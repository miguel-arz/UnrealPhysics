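; BP_PracticeTarget is a shootable practice target that shatters the first time it takes any damage.
; On BeginPlay it binds to OnTakeAnyDamage, and a DoOnce limits the break to a single hit.
; The hit swaps in the GC_BP_PracticeTarget Chaos geometry collection, hides the static mesh and disables its collision.
; A radial impulse with strain at the actor's location then fractures and scatters the pieces.
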(event `self.ReceiveBeginPlay`
  (add `self.OnTakeAnyDamage` (delegate `OnTakeAnyDamage_Event`)))

(event `OnTakeAnyDamage_Event` :!signature `self.OnTakeAnyDamage`
  (params (DamagedActor :type "Actor Object Reference") (Damage :type "Float (single-precision)") (DamageType :type "DamageType Object Reference") (InstigatedBy :type "Controller Object Reference") (DamageCauser :type "Actor Object Reference"))
  (`/Engine/EditorBlueprintResources/StandardMacros.DoOnce` false
    (:`Completed`
      (`GeometryCollectionComponent.SetRestCollection` (`self.GeometryCollection`) "/Game/Fractures/GC_BP_PracticeTarget.GC_BP_PracticeTarget" true)
      (`SceneComponent.SetHiddenInGame` (`self.StaticMesh`) true false)
      (`PrimitiveComponent.SetEnableGravity` (`self.StaticMesh`) true)
      (`PrimitiveComponent.SetCollisionEnabled` (`self.StaticMesh`) "NoCollision")
      (`PhysicsObjectBlueprintLibrary.ApplyRadialImpulse` (`self.GeometryCollection`) (`self.K2_GetActorLocation` DamagedActor) 100.0 3000.0 "RIF_Constant" true 500000.0))))

(fn `UserConstructionScript`)